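; HealthComponent is a Blueprint health component that tracks current HP against a maximum and starts at full HP on BeginPlay.
; Damage events subtract HP with a floor of zero, then fire OnDeath, which only prints, once HP reaches zero.
; Full healing resets HP to maximum, but partial healing does nothing because RestoreHp's capped-add logic is disconnected from its entry.
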(event Custom|OnHealing
  (params (Heal%20Value :type Float%20%28double-precision%29))
  (CallFunction|RestoreHp Heal%20Value))

(event Custom|OnHealingToFull
  (CallFunction|RestoreHptoFull))

(event Custom|OnTakeDamage
  (params (Value :type Float%20%28double-precision%29))
  (CallFunction|LoseHp Value)
  (CallFunction|CheckDeath))

(event Custom|OnDeath
  (Development|PrintString "Dead Event"))

(event EventBeginPlay
  (CallFunction|RestoreHptoFull))

(fn RestoreHp
  (params (Value :type Float%20%28double-precision%29)))

(fn RestoreHptoFull
  (Variables|Default|SetCurrentHp (Variables|Default|GetMaxHp))
  (Development|PrintString "Hp restored to full"))

(fn LoseHp
  (params (Value :type Float%20%28double-precision%29))
  (Variables|Default|SetCurrentHp (Math|Float|SelectFloat (- (Variables|Default|GetCurrentHp) Value) 0.0 (>= (- (Variables|Default|GetCurrentHp) Value) 0.0)))
  (Development|PrintString "Hp Lost"))

(fn CheckDeath
  (if (<= (Variables|Default|GetCurrentHp) 0.0)
    (CallFunction|OnDeath)))