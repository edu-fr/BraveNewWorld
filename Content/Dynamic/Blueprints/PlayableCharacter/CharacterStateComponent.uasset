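; Actor component that tracks a BP_Base_Character's state: horizontal speed, direction, walking, running, jumping, falling, grounded and attacking.
; BeginPlay caches the owner, its movement and animation stats components, then binds the character's movement events to flag setters.
; Tick derives speed and direction from X velocity only, refreshes falling and grounded, and overwrites walking using the walk animation threshold.
; It also draws most values as debug text every tick.
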(event Custom|OnCharacterStopRunning_Event
  ;[1 1 1] On Start Running
  (CallFunction|FinishRunning))

(event Custom|OnCharacterRun_Event
  ;[1 1 1] On Start Running
  (CallFunction|StartRunning))

(event Custom|OnCharacterWalk_Event
  ;[1 1 1] On Walk
  (CallFunction|StartWalking))

(event Custom|OnCharacterJump_Event
  ;[1 1 1] On Jump
  (CallFunction|StartJumping))

(event Custom|OnCharacterLand_Event
  (params (Hit :type Hit%20Result%20Structure))
  ;[1 1 1] On Land
  (CallFunction|FinishJumping))

(event Custom|OnCharacterStop_Event
  ;[1 1 1] On Stop
  (CallFunction|FinishWalking))

(event EventTick
  (params (DeltaSeconds :type Float%20%28single-precision%29))
  (Utilities|FlowControl|Sequence
    (:then_0
      (Utilities|UpdateVariables))
    (:then_1
      (CallFunction|DebugDrawVariablesonScreen))))

(event EventBeginPlay
  (Utilities|FlowControl|Sequence
    (:then_0
      (|SetCharacterMovementVar))
    (:then_1
      ;[1 1 1] On Jump
      (EventDispatchers|AssignOnCharacterJump (Variables|Components|GetOwner) (delegate Custom|OnCharacterJump_Event)))
    (:then_2
      ;[1 1 1] On Land
      (EventDispatchers|AssignOnCharacterLand (Variables|Components|GetOwner) (delegate Custom|OnCharacterLand_Event)))
    (:then_3
      ;[1 1 1] On Walk
      (EventDispatchers|BindEventtoOnCharacterWalk (Variables|Components|GetOwner) (delegate Custom|OnCharacterWalk_Event)))
    (:then_4
      ;[1 1 1] On Stop
      (EventDispatchers|BindEventtoOnCharacterStop (Variables|Components|GetOwner) (delegate Custom|OnCharacterStop_Event)))
    (:then_5
      ;[1 1 1] On Start Running
      (EventDispatchers|BindEventtoOnCharacterRun (Variables|Components|GetOwner) (delegate Custom|OnCharacterRun_Event)))
    (:then_6
      ;[1 1 1] On Start Running
      (EventDispatchers|BindEventtoOnCharacterStopRunning (Variables|Components|GetOwner) (delegate Custom|OnCharacterStopRunning_Event)))))

(fn DebugDrawVariablesonScreen
  (Utilities|FlowControl|Sequence
    (:then_0
      (CallFunction|DebugDrawVariable 0 "CurrentHorizontalSpeed" (Math|Float|Truncate (Variables|Default|GetCurrentHorizontalSpeed))))
    (:then_1
      (CallFunction|DebugDrawVariable 1 "CurrentNormalizedDirection" (Variables|Default|GetCurrentNormalizedDirection)))
    (:then_2
      (CallFunction|DebugDrawVariable 2 "IsWalking?" (Math|Conversions|ToInteger(Boolean) (Variables|Default|GetIsWalking))))
    (:then_3
      (CallFunction|DebugDrawVariable 3 "IsRunning?" (Math|Conversions|ToInteger(Boolean) (Variables|Default|GetIsRunning))))
    (:then_4
      (CallFunction|DebugDrawVariable 4 "IsAttacking?" (Math|Conversions|ToInteger(Boolean) (Variables|Default|GetIsAttacking))))
    (:then_5
      (CallFunction|DebugDrawVariable 5 "IsGrounded?" (Math|Conversions|ToInteger(Boolean) (Variables|Default|GetIsGrounded))))
    (:then_6
      (CallFunction|DebugDrawVariable 6 "IsFalling?" (Math|Conversions|ToInteger(Boolean) (Variables|Default|GetIsFalling))))))

(fn DebugDrawVariable
  (params (Var%20Number :type Integer) (Name :type String) (Value :type Integer))
  (bind _boxextent_z (|ActorHeight))
  (bind _returnvalue_z (|ActorLocation))
  (bind _returnvalue (* Var%20Number -10))
  (bind _self self)
  (bind _returnvalue_2 (Components|GetOwner _self))
  (bind _returnvalue_3 (- _returnvalue _boxextent_z))
  (bind _returnvalue_4 (- _returnvalue_3 _returnvalue_z))
  (Rendering|Debug|DrawDebugString (Math|Vector|MakeVector -75.0 0.0 _returnvalue_4) (Utilities|String|ToString(Integer) Value) _returnvalue_2 "(R=1.000000,G=1.000000,B=1.000000,A=1.000000)")
  (Rendering|Debug|DrawDebugString (Math|Vector|MakeVector 75.0 0.0 _returnvalue_4) Name _returnvalue_2 "(R=1.000000,G=1.000000,B=1.000000,A=1.000000)"))

(fn ShouldMove?
  (return (and (> (Variables|Default|GetCurrentHorizontalSpeed) 3.0) (!= (.x (Pawn|Components|CharacterMovement|GetCurrentAcceleration (Variables|Default|GetCharacterMovement))) 0.0))))

(fn StartJumping
  (Variables|Default|SetIsJumping true))

(fn FinishJumping
  (params (Hit :type Hit%20Result%20Structure))
  (Variables|Default|SetIsJumping false)
  (Variables|Default|SetIsGrounded true))

(fn StartWalking
  (Variables|Default|SetIsWalking true))

(fn FinishWalking
  (Variables|Default|SetIsWalking false)
  (CallFunction|FinishWalking))

(fn StartRunning
  (Variables|Default|SetIsRunning true))

(fn FinishRunning
  (Variables|Default|SetIsRunning false)
  (Development|PrintString "Finished running"))

(fn StartAttacking
  (Variables|Default|SetIsAttacking true))

(fn FinishAttacking
  (Variables|Default|SetIsAttacking false))