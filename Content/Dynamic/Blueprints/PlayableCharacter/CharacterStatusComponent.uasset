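; Character component that tracks the movement and action state of its BP_Base_Character owner.
; It caches the movement and animation stats components, then each Tick updates speed, direction, falling and walking, with walking derived from an animation threshold.
; Horizontal speed is signed X velocity only, so ShouldMove and the walk check pass only for positive X.
; Start/Finish functions set jump, walk, run and attack flags, though StartRunning sets IsRunning false.
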(event EventBeginPlay
  (|SetCharacterMovementVar))

(event EventTick
  (params (DeltaSeconds :type Float%20%28single-precision%29))
  (Utilities|UpdateVariables))

(fn ShouldMove?
  (return (and (> (Variables|Default|GetCurrentHorizontalSpeed) 3.0) (!= (.x (Pawn|Components|CharacterMovement|GetCurrentAcceleration (Variables|Default|GetCharacterMovement))) 0.0))))

(fn StartJumping
  (Variables|Default|SetIsJumping true)
  (Variables|Default|SetIsGrounded false))

(fn FinishJumping
  (Variables|Default|SetIsJumping false))

(fn StartWalking
  (Variables|Default|SetIsWalking true))

(fn FinishWalking
  (Variables|Default|SetIsWalking false))

(fn StartRunning
  (Variables|Default|SetIsRunning false))

(fn FinishRunning
  (Variables|Default|SetIsRunning false))

(fn StartAttacking
  (Variables|Default|SetIsAttacking true))

(fn FinishAttacking
  (Variables|Default|SetIsAttacking false))