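; Health component that tracks an owner's current and max HP, handling damage, healing and death.
; BeginPlay and HealToFull restore HP to max, while Heal and TakeDamage adjust it through helper functions that clamp at max or zero and print debug strings.
; Every change broadcasts OnHpChanged with current and max HP, and damage that leaves HP at zero calls Die, which broadcasts OnDeath.
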(event Custom|HealToFull
  ;[1 1 1] Events
  (bind _newvalue (CallFunction|RestoreHptoFull))
  (Default|CallOnHpChanged _newvalue (Variables|Default|GetMaxHp)))

(event Custom|TakeDamage
  (params (Value :type Float%20%28double-precision%29))
  ;[1 1 1] Events
  (bind __newvalue (CallFunction|LoseHp Value))
  (Default|CallOnHpChanged __newvalue (Variables|Default|GetMaxHp))
  (bind _dead (CallFunction|CheckDeath))
  (if _dead
    (CallFunction|Die)))

(event Custom|Die
  ;[1 1 1] Events
  (Default|CallOnDeath))

(event Custom|Heal
  (params (Heal%20Value :type Float%20%28double-precision%29))
  ;[1 1 1] Events
  (bind _newvalue (CallFunction|RestoreHp Heal%20Value))
  (Default|CallOnHpChanged _newvalue (Variables|Default|GetMaxHp)))

(event EventBeginPlay
  ;[1 1 1] BeginPlay
  ;[1 1 1] Events
  (bind _newvalue (CallFunction|RestoreHptoFull))
  (Default|CallOnHpChanged _newvalue (Variables|Default|GetMaxHp)))

(fn RestoreHp
  (params (Value :type Float%20%28double-precision%29))
  (bind _maxhp (Variables|Default|GetMaxHp))
  (bind _output_get (Variables|Default|SetCurrentHp (Math|Float|SelectFloat (+ Value (Variables|Default|GetCurrentHp)) _maxhp (<= (+ Value (Variables|Default|GetCurrentHp)) _maxhp))))
  (Development|PrintString "Healed")
  (return _output_get))

(fn RestoreHptoFull
  (bind _output_get (Variables|Default|SetCurrentHp (Variables|Default|GetMaxHp)))
  (Development|PrintString "Hp restored to full")
  (return _output_get))

(fn LoseHp
  (params (HpToLose :type Float%20%28double-precision%29))
  (bind _output_get (Variables|Default|SetCurrentHp (Math|Float|SelectFloat (- (Variables|Default|GetCurrentHp) HpToLose) 0.0 (>= (- (Variables|Default|GetCurrentHp) HpToLose) 0.0))))
  (Development|PrintString "Hp Lost")
  (return _output_get))

(fn CheckDeath
  (return (<= (Variables|Default|GetCurrentHp) 0.0)))