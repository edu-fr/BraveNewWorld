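; BP_CameraManager is a follow camera actor that smoothly trails a FollowTarget.
; Each Tick, UpdateCameraPos uses VInterpTo to move it toward the target's position plus a forward-vector offset applied only on X and Z.
; LockHeight keeps the camera's current Z as the base height instead of the target's.
; It prints debug messages when the target is invalid or the camera is destroyed.
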(event EventDestroyed
  (Development|PrintString "Camera destroyed"))

(event EventTick
  (params (DeltaSeconds :type Float%20%28single-precision%29))
  (CallFunction|UpdateCameraPos))

(fn ConstructionScript)

(fn UpdateCameraPos
  (bind _camoffset (Variables|Default|GetCamOffset))
  (bind _followtarget (Variables|Default|GetFollowTarget))
  (bind _followtarget_2 (Variables|Default|GetFollowTarget))
  (bind _returnvalue (Transformation|GetActorForwardVector _followtarget))
  (bind _returnvalue_2 (Transformation|GetActorLocation _followtarget_2))
  (bind _returnvalue_3 (* _returnvalue _camoffset))
  (Utilities|IsValid (Variables|Default|GetFollowTarget)
    (:Is%20Valid
      ;[1 1 1] SetCameraPos
      (Transformation|SetActorLocation (Math|Interpolation|VInterpTo (Transformation|GetActorLocation) (+ (Math|Vector|MakeVector (.x _returnvalue_2) (.y _returnvalue_2) (Math|Float|SelectFloat (.z (Transformation|GetActorLocation)) (.z _returnvalue_2) (Variables|Default|GetLockHeight))) (Math|Vector|MakeVector (.x _returnvalue_3) 0.0 (.z _returnvalue_3))) (Utilities|Time|GetWorldDeltaSeconds) (Variables|Default|GetInterpSpeed)) false false))
    (:Is%20Not%20Valid
      (Development|PrintString "Invalid Camera Follow Actor" true true "(R=1.000000,G=0.000000,B=0.000000,A=1.000000)"))))