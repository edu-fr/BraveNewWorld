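; BP_Enemy_Spawner is an enemy spawner that replaces its enemy whenever that enemy dies.
; On BeginPlay, if ShouldSpawn is set, it starts a spawn cycle that creates a BP_Base_EnemyCharacter at the spawner's world transform.
; Each cycle binds to the new enemy's OnCharacterDeath dispatcher, which immediately starts the next cycle with no delay or count limit.
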(event Custom|Spawn%20Cycle
  ;[1 1 1] Spawn Cycle
  (bind _enemyspawned (CallFunction|SpawnEnemy))
  (EventDispatchers|AssignOnCharacterDeath _enemyspawned (delegate Custom|OnCharacterDeath_Event)))

(event Custom|OnCharacterDeath_Event
  ;[1 1 1] Spawn Cycle
  (CallFunction|SpawnCycle))

(event EventBeginPlay
  (if (Variables|Default|GetShouldSpawn)
    (CallFunction|SpawnCycle)))

(fn SpawnEnemy
  (bind _returnvalue (Game|SpawnActorfromClass "/Game/Dynamic/Blueprints/Enemy/BP_Base_EnemyCharacter.BP_Base_EnemyCharacter_C" (Transformation|GetWorldTransform) "Undefined" "MultiplyWithRoot" 0 0))
  (return _returnvalue))