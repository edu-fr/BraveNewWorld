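; Enemy AI state machine component that switches an enemy between idle, chasing, attacking and submissive states.
; After Init injects owner, search collider, stats and debug text, a half-second tick selects a target from overlapping playable characters and runs range checks.
; Attacks play the owner's animation, then a timer using its returned duration restores chasing.
; State changes broadcast and print; chase movement is disabled and submissive recovery is a stub.
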(event EventBeginPlay
  (Class|ActorComponent|SetComponentTickInterval 0.5))

(event EventTick
  (params (DeltaSeconds :type Float%20%28single-precision%29))
  (if (Variables|Default|GetDidInit)
    (CallFunction|StateMachineTick)))

(fn Init
  (params (Owner :type BP%20Base%20Enemy%20Character%20Object%20Reference) (SearchCollider :type Sphere%20Component%20Object%20Reference) (CharacterStats :type Character%20Stats%20Component%20Object%20Reference) (StateTextDebug :type Text%20Render%20Component%20Object%20Reference))
  ;[1 1 1] Setup variables
  (Variables|Default|SetOwnerBaseEnemy Owner)
  (Variables|Default|SetSearchCollider SearchCollider)
  (Variables|Default|SetCharacterStats CharacterStats)
  ;[1 1 1] Setup debug
  (Variables|Default|SetStateTextDebug StateTextDebug)
  (Variables|Default|SetDidInit true))

(fn StateMachineTick
  (if (Variables|Default|GetDidInit)
    (switch Utilities|FlowControl|Switch|SwitchonEnemy_States (Variables|Default|GetCurrentState)
      (:NewEnumerator0
        ;[1 1 1] Idle
        (bind _playerfound (CallFunction|LookforPlayers))
        (if _playerfound
          (CallFunction|StartChasing)
          (CallFunction|ChangeState "NewEnumerator1")))
      (:NewEnumerator1
        ;[1 1 1] Chasing
        (if (Utilities|CheckContinueChasing)
          (if (Utilities|CheckCanAttack)
            ;;[1 1 1] Start attack because player in enough range
            (CallFunction|ChangeState "NewEnumerator2"))
          (else
            ;;[1 1 1] Cancel chase because player is out of range
            (CallFunction|ChangeState "NewEnumerator0"))))
      (:NewEnumerator2
        ;[1 1 1] StartAttack
        (bind _attackanimationduration (CallFunction|AttackPlayer))
        (CallFunction|ChangeState "NewEnumerator4")
        ;;[1 1 1] Back to chasing after attacking
        (Utilities|Time|SetTimerbyFunctionName 0 "ChangeToChasingState" _attackanimationduration))
      (:NewEnumerator3
        ;[1 1 1] Submissive
        (CallFunction|TrytoGetBacktoCombat)
        (if true
          (CallFunction|ChangeState "NewEnumerator1"))))))

(fn ChangeState
  (params (NewState :type Enemy_States%20Enum :default "NewEnumerator0"))
  (bind _output_get (Variables|Default|SetPreviousState (Variables|Default|GetCurrentState)))
  (bind _output_get_2 (Variables|Default|SetCurrentState NewState))
  (Default|CallOnStateChanged _output_get_2 _output_get)
  ;[1 1 1] Debug
  (Rendering|Components|TextRender|SetText (Variables|Default|GetStateTextDebug) (Utilities|Text|ToText(String) (Utilities|String|EnumtoString _output_get_2)))
  (Development|PrintString (Utilities|String|ToString(Text) (Utilities|Text|ToText(String) (Utilities|String|EnumtoString _output_get_2)))))

(fn LookforPlayers
  (bind _closestplayablecharacter (Utilities|GetClosestPlayableCharacterinColliderRange (Variables|Default|GetSearchCollider))
    (:End
      (bind _output_get (Variables|Default|SetPlayerToChase _closestplayablecharacter))
      (Utilities|IsValid _output_get
        (:Is%20Valid
          (return true))
        (:Is%20Not%20Valid
          (return false))))))

(fn AttackPlayer
  (bind _animationduration (Default|DoAttackAnimation (Variables|Default|GetOwnerBaseEnemy)))
  (return _animationduration))

(fn TrytoGetBacktoCombat
  (return true))

(fn PlayerStillinRange
  (Utilities|IsValid (Variables|Default|GetPlayerToChase)
    (:Is%20Valid
      (return (<= (Utilities|GetDistancefromPlayer) (Variables|/Game/Dynamic/Blueprints/PlayableCharacter/CharacterStatsComponent.CharacterStatsComponent_C|GetOutOfChaseRange (Variables|Default|GetCharacterStats)))))
    (:Is%20Not%20Valid
      (return false))))

(fn StartChasing
  (if (not true)
    (AI|Navigation|SimpleMovetoActor (AI|GetAIController (Variables|Default|GetOwnerBaseEnemy)) (Variables|Default|GetPlayerToChase))))

(fn ChangetoChasingState
  (CallFunction|ChangeState "NewEnumerator1"))