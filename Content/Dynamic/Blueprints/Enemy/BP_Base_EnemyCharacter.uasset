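; Base enemy character Blueprint that connects an enemy's health component to its health bar widget.
; On BeginPlay it casts the widget component's widget to WB_Enemy_HealthBar and binds an event to the HP-changed notification, printing a red error if the cast fails.
; The parent BeginPlay runs after this binding.
; GetBlackBoard holds only an unconnected lookup of the AI controller's blackboard, and the construction script just calls its parent.
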(event EventBeginPlay
  (Utilities|FlowControl|Sequence
    (:then_0
      ;[1 1 1] Binding Health Bar Update
      (bind _aswb_enemy_health_bar (Utilities|Casting|CastToWB_Enemy_HealthBar (UserInterface|GetWidget (Variables|Default|GetEnemy%20Health%20Bar%20Widget)))
        (:then
          (EventDispatchers|BindEventtoOnHpChanged (Variables|Default|GetHealthComponent) (EventDispatchers|CreateEvent _aswb_enemy_health_bar :!event UpdateEnemyHpBar)))
        (:CastFailed
          (Development|PrintString "Error casting enemy health bar class" true true "(R=1.000000,G=0.000000,B=0.000000,A=1.000000)"))))
    (:then_2
      (|CallParentFunction))))

(fn ConstructionScript
  (|CallParentFunction))