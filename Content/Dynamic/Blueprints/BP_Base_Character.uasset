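; Base character Blueprint for sword combat, providing shared attack, hit reaction, death, walk/run and facing logic.
; Hit detection sphere-traces pawns at the right-hand socket, ignoring actors already hit this attack, then calls HitReact on struck characters.
; HitReact plays a montage and damages the HealthComponent, whose death event broadcasts and destroys the actor.
; BeginPlay draws the sword, CharacterStatsComponent supplies movement speeds, and SetRotation smoothly flips yaw between two opposite directions.
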(event Custom|HitReact
  (params (HitDamage :type Float%20%28double-precision%29))
  ;[1 1 1] Hit React
  (Animation|Montage|PlayMontage (Variables|Character|GetMesh) "/Game/Static/Characters/Mannequins/Animations/Manny/Combat/Reaction/Custom_Head_Hit_Montage.Custom_Head_Hit_Montage"
    (:then
      (Default|TakeDamage (Variables|Default|GetHealthComponent) HitDamage))))

(event Custom|HitDetect
  (bind _mesh (Variables|Character|GetMesh))
  (bind _returnvalue (Transformation|GetSocketLocation _mesh "onehanded_r"))
  ;[1 1 1] Hit Detect
  (bind _outhit (Collision|SphereTraceForObjects _returnvalue _returnvalue 5e+01 (Utilities|Array|MakeArray "ObjectTypeQuery3") false (Variables|Default|GetActorsHitByCurrentAttack) "ForDuration"))
  (bind _asbp_base_character (Utilities|Casting|CastToBP_Base_Character (.HitActor (Collision|BreakHitResult _outhit))))
  (Utilities|Array|AddUnique (Variables|Default|GetActorsHitByCurrentAttack) (.HitActor (Collision|BreakHitResult _outhit)))
  (CallFunction|HitReact _asbp_base_character (Variables|Default|GetWeaponDamage)))

(event Custom|NewAttackAnimationStarted
  ;[1 1 1] Clear Hit Detection List
  (Utilities|Array|Clear (Variables|Default|GetActorsHitByCurrentAttack)))

(event Custom|DeathBehavior
  ;[1 1 1] Death Behavior
  (Default|CallOnCharacterDeath)
  (Actor|DestroyActor))

(event EventBeginPlay
  ;[1 1 1] Begin Play
  (Utilities|FlowControl|Sequence
    (:then_0
      ;;[1 1 1] Bind on death event
      (EventDispatchers|BindEventtoOnDeath (Variables|Default|GetHealthComponent) (delegate Custom|DeathBehavior)))
    (:then_1
      ;;[1 1 1] Equip weapon on Start
      (Animation|PlayAnimMontage "/Game/Static/Characters/Mannequins/Animations/Manny/Combat/Preparation/Custom_Draw_Sword_Montage.Custom_Draw_Sword_Montage" 1.0 "None"))))

(fn ConstructionScript)

(fn SetRotation
  (params (A :type Float%20%28double-precision%29))
  (Transformation|SetActorRotation (Math|Interpolation|RInterpTo (Transformation|GetActorRotation) (Math|Rotator|MakeRotator 0.0 0.0 (.z (Math|Vector|SelectVector "0.000000,0.000000,180.000000" "0, 0, 0" (> A 0.0)))) (Utilities|Time|GetWorldDeltaSeconds) 0.0)))

(fn DoAttackAnimation
  ;[1 1 1] Attack Animation
  (bind _returnvalue (Animation|PlayAnimMontage "/Game/Static/Characters/Mannequins/Animations/Manny/Combat/Attack/Custom_Attack_Sword_Montage.Custom_Attack_Sword_Montage" 1.0 "None"))
  (return _returnvalue))

(fn StartRunning
  (Variables|/Script/Engine.CharacterMovementComponent|SetMaxWalkSpeed (Variables|Character|GetCharacterMovement) (Variables|/Game/Dynamic/Blueprints/PlayableCharacter/CharacterStatsComponent.CharacterStatsComponent_C|GetRunning%20Speed (Variables|Default|GetCharacterStatsComponent)))
  (Variables|Default|SetIsRunning true))

(fn StopRunning
  (Variables|/Script/Engine.CharacterMovementComponent|SetMaxWalkSpeed (Variables|Character|GetCharacterMovement) (Variables|/Game/Dynamic/Blueprints/PlayableCharacter/CharacterStatsComponent.CharacterStatsComponent_C|GetWalking%20Speed (Variables|Default|GetCharacterStatsComponent)))
  (Variables|Default|SetIsRunning false))